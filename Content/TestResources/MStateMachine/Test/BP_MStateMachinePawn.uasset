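; Test pawn that exercises the MStateMachine component with keyboard-driven movement states.
; On BeginPlay it registers Idle, Walk and Dash state definitions, sets the Look action as entry state and starts ticking.
; W switches between Walk and Look, while Left Shift requests Run during walking and returns to Walk or Look on release.
; The Run request prints whether the switch succeeded; the pawn's graph only requests states and applies no movement.
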(event `self.ReceiveBeginPlay`
  (bind _mstatemachine (`self.MStateMachine`))
  (`MStateMachineComponent.AddNewState` (`self.MStateMachine`) "/Game/TestResources/MStateMachine/Test/BP_MStateDefinition_Idle.BP_MStateDefinition_Idle_C")
  (`MStateMachineComponent.AddNewState` (`self.MStateMachine`) "/Game/TestResources/MStateMachine/Test/BP_MStateDefinition_Walk.BP_MStateDefinition_Walk_C")
  (`MStateMachineComponent.AddNewState` _mstatemachine "/Game/TestResources/MStateMachine/Test/BP_MStateDefinition_Dash.BP_MStateDefinition_Dash_C")
  (`MStateMachineComponent.SetEntryState` _mstatemachine (struct :`TagName` "CHAbility.Action.Look"))
  (`MStateMachineComponent.StartTickState` (`self.MStateMachine`)))

(event `Key|W`
  (params (Key :type "Key Structure"))
  (bind _mstatemachine (`self.MStateMachine`))
  (:`Pressed`
    (set `self.bIsWalk` true)
    (`MStateMachineComponent.SwitchNextState` _mstatemachine (struct :`TagName` "CHAbility.Action.Walk")))
  (:`Released`
    (set `self.bIsWalk` false)
    (`MStateMachineComponent.SwitchNextState` _mstatemachine (struct :`TagName` "CHAbility.Action.Look"))))

(event `Key|LeftShift`
  (params (Key :type "Key Structure"))
  (:`Pressed`
    (set `self.bIsHoldRun` true)
    (if (`self.bIsWalk`)
      (bind _returnvalue (`MStateMachineComponent.SwitchNextState` (`self.MStateMachine`) (struct :`TagName` "CHAbility.Action.Run")))
      (if _returnvalue
        (`KismetSystemLibrary.PrintString` "Success")
        (else
          (`KismetSystemLibrary.PrintString` "Failed")))))
  (:`Released`
    (set `self.bIsHoldRun` false)
    (if (`self.bIsWalk`)
      (`MStateMachineComponent.SwitchNextState` (`self.MStateMachine`) (struct :`TagName` "CHAbility.Action.Walk"))
      (else
        (`MStateMachineComponent.SwitchNextState` (`self.MStateMachine`) (struct :`TagName` "CHAbility.Action.Look"))))))

(fn `UserConstructionScript`)