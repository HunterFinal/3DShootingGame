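; BP_GASTestPawn is a test pawn for exercising the Gameplay Ability System.
; On BeginPlay it grants two print-string test abilities, GA_PrintString and GA_PrintAnotherString, to its AbilitySystem component.
; Left and right mouse buttons try to activate abilities by tag, using the melee action and shooting aim tags respectively, with remote activation allowed.
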(event `self.ReceiveBeginPlay`
  (`AbilitySystemComponent.K2_GiveAbility` (`self.AbilitySystem`) "/Game/TestResources/GA_PrintString.GA_PrintString_C" 0 -1)
  (`AbilitySystemComponent.K2_GiveAbility` (`self.AbilitySystem`) "/Game/TestResources/GA_PrintAnotherString.GA_PrintAnotherString_C" 0 -1))

(event `Key|LeftMouseButton`
  (params (Key :type "Key Structure"))
  (:`Pressed`
    (`AbilitySystemComponent.TryActivateAbilitiesByTag` (`self.AbilitySystem`) (`BlueprintGameplayTagLibrary.MakeGameplayTagContainerFromTag` (struct :`TagName` "CHAbility.Action.Melee")) true)))

(event `Key|RightMouseButton`
  (params (Key :type "Key Structure"))
  (:`Pressed`
    (`AbilitySystemComponent.TryActivateAbilitiesByTag` (`self.AbilitySystem`) (`BlueprintGameplayTagLibrary.MakeGameplayTagContainerFromTag` (struct :`TagName` "CHAbility.Shooting.Aim")) true)))

(fn `UserConstructionScript`)