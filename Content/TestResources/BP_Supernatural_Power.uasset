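; BP_Supernatural_Power is a test Blueprint for a wall-hack vision power that switches the materials of hackable actors.
; SwitchMat_Event flips IsHacking, then gathers every actor implementing BP_IWallHackable.
; It passes each one OcclusionMat or NormalMat through SetWallHackMat, so each actor applies the change through the interface.
; BeginPlay, Tick, overlap and the construction script are empty.
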(event `SwitchMat_Event`
  (set `self.IsHacking` (not (`self.IsHacking`)))
  (bind _outactors (`GameplayStatics.GetAllActorsWithInterface` "/Game/TestResources/BP_IWallHackable.BP_IWallHackable_C"))
  (for _array_element _outactors
    (bind _asbp_iwall_hackable (cast `/Game/TestResources/BP_IWallHackable` _array_element))
    (if (`self.IsHacking`)
      (`/Game/TestResources/BP_IWallHackable.SetWallHackMat` _asbp_iwall_hackable (`self.OcclusionMat`))
      (else
        (`/Game/TestResources/BP_IWallHackable.SetWallHackMat` _asbp_iwall_hackable (`self.NormalMat`))))))

(fn `UserConstructionScript`)