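; BP_CheatEffectPlayer_TEST is a test player Blueprint for moving around and triggering material switches on BP_Supernatural_Power actors.
; W and S set forward and backward scales, which Tick sums and feeds into AddMovementInput along the actor's forward vector.
; Pressing 1 finds every BP_Supernatural_Power in the level and calls SwitchMatEvent on each.
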(event `self.ReceiveTick`
  (params (DeltaSeconds :type "Float (single-precision)"))
  (`self.AddMovementInput` (`self.GetActorForwardVector`) (+ (`self.MoveForwardScale`) (`self.MoveBackwardScale`))))

(event `Key|W`
  (params (Key :type "Key Structure"))
  (:`Pressed`
    (set `self.MoveForwardScale` 1.0))
  (:`Released`
    (set `self.MoveForwardScale` 0.0)))

(event `Key|S`
  (params (Key :type "Key Structure"))
  (:`Pressed`
    (set `self.MoveBackwardScale` -1.0))
  (:`Released`
    (set `self.MoveBackwardScale` 0.0)))

(event `Key|One`
  (params (Key :type "Key Structure"))
  (:`Pressed`
    (bind _outactors (`GameplayStatics.GetAllActorsOfClass` "/Game/TestResources/BP_Supernatural_Power.BP_Supernatural_Power_C"))
    (for _array_element _outactors
      (`/Game/TestResources/BP_Supernatural_Power.SwitchMat_Event` _array_element))))

(fn `UserConstructionScript`)